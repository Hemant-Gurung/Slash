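; BP_EnemyChar is an axe-wielding melee enemy that chases and attacks the player.
; On BeginPlay it spawns BP_AxeEnemy onto its hand socket, and pawn sensing starts an AI MoveTo toward the seen player.
; Tick checks 2D distance to the player, stopping movement and playing a delayed slash montage when close.
; BPC_Health's death event plays montage and sound, then destroys enemy and weapon.
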(event `self.ReceiveBeginPlay`
  ;[1 1 1] Spawn Enemy Weapon in the beginning
  (bind _returnvalue (`|SpawnActorFromClass` "/Game/Blueprints/BP_AxeEnemy.BP_AxeEnemy_C" (`SceneComponent.K2_GetComponentToWorld` (`self.Mesh`)) "Undefined" "OverrideRootScale" null null))
  (bind _output_get (set `self.currentWeaponEnemy` _returnvalue))
  (`self.K2_AttachToComponent` _output_get (`self.Mesh`) "enemySword" "SnapToTarget" "SnapToTarget" "KeepRelative" true))

(event `self.EnemySense.OnSeePawn`
  (params (Pawn :type "Pawn Object Reference"))
  (bind _asbp_player_char (cast `/Game/Blueprints/BP_PlayerChar` Pawn))
  (`|AIMoveTo` self (`SceneComponent.K2_GetComponentLocation` (`Character.Mesh` (`GameplayStatics.GetPlayerCharacter` 0))) _asbp_player_char 20.0))

(event `self.ReceiveTick`
  (params (DeltaSeconds :type "Float (single-precision)"))
  ;[1 1 1] check if playre is near
  (`|ExecutionSequence`
    (:`then_0`
      (if (< (`KismetMathLibrary.Vector_Distance2D` (`SceneComponent.K2_GetComponentLocation` (`self.Mesh`)) (`SceneComponent.K2_GetComponentLocation` (`Character.Mesh` (`GameplayStatics.GetPlayerCharacter` 0)))) 200.0)
        (set `self.IsPlayerNear` true)
        (set `CharacterMovementComponent.MaxWalkSpeed` 0.0 (`self.CharacterMovement`))
        (`KismetSystemLibrary.Delay` 1.0)
        (if (not (`self.isDead`))
          (`self.PlayAnimMontage` "/Game/Animations/Animations/EnemySlashMontage.EnemySlashMontage")
          (`KismetSystemLibrary.Delay` 2.0))
        (else
          (set `self.IsPlayerNear` false)
          (set `CharacterMovementComponent.MaxWalkSpeed` 600.0 (`self.CharacterMovement`)))))))

(event `self.BPC_Health.onDeath`
  (set `self.isDead` true)
  (set `CharacterMovementComponent.MaxWalkSpeed` 0.0 (`self.CharacterMovement`))
  (`self.PlayAnimMontage` "/Game/Animations/Animations/Anime_montage_death.Anime_montage_death")
  (`GameplayStatics.PlaySoundAtLocation` "/Game/Sounds/EnemySounds/Cue_EnemyDeathSound.Cue_EnemyDeathSound" (`SceneComponent.K2_GetComponentLocation` (`self.Mesh`)) (struct) 1.0 1.0 0.0 null null null)
  (`KismetSystemLibrary.Delay` 3.0)
  (`self.K2_DestroyActor`)
  (`self.K2_DestroyActor` (`self.currentWeaponEnemy`)))

(event `IsHurt`
  (if (not (`self.isDead`))
    (`KismetSystemLibrary.Delay` 0.5)))

(fn `UserConstructionScript`)