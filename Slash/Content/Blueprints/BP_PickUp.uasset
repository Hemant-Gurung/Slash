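; BP_PickUp is a pickup actor with a Cube mesh and a Widget component, driven entirely from Tick.
; When the player character is within a fixed range, it rotates the widget to face them, but both range branches hide the widget, so this graph never shows it.
; Every tick it also enables custom depth rendering on the cube, regardless of distance.
; The graph contains no collection or overlap logic.
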(event `self.ReceiveTick`
  (params (DeltaSeconds :type "Float (single-precision)"))
  (`|ExecutionSequence`
    (:`then_0`
      ;[1 1 1] Widget rotattion
      (if (< (`KismetMathLibrary.VSize` (- (`self.K2_GetActorLocation` (`GameplayStatics.GetPlayerCharacter` 0)) (`self.K2_GetActorLocation`))) 350.0)
        (`SceneComponent.SetVisibility` (`self.Widget`) false false)
        (`SceneComponent.K2_SetWorldRotation` (`self.Widget`) (`KismetMathLibrary.FindLookAtRotation` (`self.K2_GetActorLocation`) (`self.K2_GetActorLocation` (`GameplayStatics.GetPlayerCharacter` 0))) false false)
        (else
          (`SceneComponent.SetVisibility` (`self.Widget`) false false))))
    (:`then_1`
      (bind _output_get (set `self.IsCustomDepthSet` true))
      (`PrimitiveComponent.SetRenderCustomDepth` (`self.Cube`) _output_get))))

(fn `UserConstructionScript`)