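; BPC_Health is a health component that tracks current health against a maximum and signals death.
; Health resets to the maximum on BeginPlay or through the ResetHealth event.
; DoDamage clamps health between zero and the maximum, then returns whether the owner is dead via IsDead, which tests the health percentage against zero.
; It calls OnDeath only when that hit actually lowered health to zero, so repeated damage does not retrigger it.
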(event `self.ReceiveBeginPlay`
  (`self.ResetHealth`))

(event `ResetHealth`
  (set `self.currentHealth` (`self.maxHealth`)))

(fn `DoDamage`
  (params (damageAmount :type "Float (double-precision)"))
  (returns (isDead :type Boolean))
  (locals (OriginalHealth :type "Float (double-precision)"))
  (bind _isdead (`self.IsDead`))
  (set `local.OriginalHealth` (`self.currentHealth`))
  (bind _output_get (set `self.currentHealth` (`KismetMathLibrary.FClamp` (- (`self.currentHealth`) damageAmount) 0.0 (`self.maxHealth`))))
  ;[1 1 1] did this do damage cause the health to drop to 0
  (if (and _isdead (> (`local.OriginalHealth`) _output_get))
    (`self.onDeath`))
  (return _isdead))

(fn `GetHealthPercentage`
  (returns (`Health Percentage` :type "Float (double-precision)"))
  (return (/ (`self.currentHealth`) (`self.maxHealth`))))

(fn `IsDead`
  (returns (IsDead :type Boolean))
  (return (== (`self.GetHealthPercentage`) 0.0)))