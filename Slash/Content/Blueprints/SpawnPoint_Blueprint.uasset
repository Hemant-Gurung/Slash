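; A checkpoint actor that updates the player's respawn point when the player walks into its trigger.
; On overlap by BP_PlayerChar, it sets that character's Respawn transform to the trigger's location, raised slightly, with the trigger's rotation and unit scale.
; It then plays a portal sound and shows a BPW_Checkpoint widget carrying its CheckpointInfo, removing it after a short delay.
; Nothing gates repeat activation.
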(event `self.CheckpoointTrigger.OnComponentBeginOverlap`
  (params (OverlappedComponent :type "PrimitiveComponent Object Reference") (OtherActor :type "Actor Object Reference") (OtherComp :type "PrimitiveComponent Object Reference") (OtherBodyIndex :type Integer) (bFromSweep :type Boolean) (SweepResult :type "HitResult Structure (by ref)"))
  (bind (_returnvalue_location _returnvalue_rotation) (`KismetMathLibrary.BreakTransform` (`SceneComponent.K2_GetComponentToWorld` (`self.CheckpoointTrigger`))))
  ;[1 1 1] respawn function
  (bind _asbp_player_char (cast `/Game/Blueprints/BP_PlayerChar` OtherActor))
  (set `/Game/Blueprints/BP_PlayerChar.Respawn` (`KismetMathLibrary.MakeTransform` (+ _returnvalue_location (0.0 0.0 140.0)) _returnvalue_rotation) _asbp_player_char)
  (`GameplayStatics.PlaySound2D` "/Game/Sounds/PortalEntry.PortalEntry" 1.0 1.0 0.0 null null)
  (bind _returnvalue (`|CreateWidget` "/Game/Blueprints/BPW_Checkpoint.BPW_Checkpoint_C"))
  (set `/Game/Blueprints/BPW_Checkpoint.CheckpointInfo` (`self.Checkpoint Info`) _returnvalue)
  (`UserWidget.AddToViewport` _returnvalue 0)
  (`KismetSystemLibrary.Delay` 2.0)
  (`Widget.RemoveFromParent` _returnvalue))

(fn `UserConstructionScript`)