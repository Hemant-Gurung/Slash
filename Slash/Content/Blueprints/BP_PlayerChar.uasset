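; Player character with an equippable sword that can slash, be thrown and be recalled, plus physics-handle object pickup.
; A socket-to-camera-forward trace sets the throw target, and Tick moves and spins the detached sword toward it.
; Recall offsets the return target along the sword's right vector for a curved path, then reattaches it with shake and sound.
; BPC_Health death triggers a delayed respawn, possessing a newly spawned character.
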(event `self.ReceiveBeginPlay`
  ;[1 1 1] Attach sword in the beginning
  (`|ExecutionSequence`
    (:`then_0`
      (bind _returnvalue (`|SpawnActorFromClass` "/Game/Blueprints/BP_SwordMihwak.BP_SwordMihwak_C" (`SceneComponent.K2_GetComponentToWorld` (`self.Mesh`)) "Undefined" "OverrideRootScale" null null))
      (bind _output_get (set `self.currentWeapon` _returnvalue))
      (`self.K2_AttachToComponent` _output_get (`self.Mesh`) "unshealthed" "SnapToTarget" "SnapToTarget" "KeepRelative" true)
      (set `self.isHoldingObject` true))))

(event `swing`
  (bind _charactermovement (`self.CharacterMovement`))
  ;[1 1 1] SwingSword Trigger Mouse Button
  (if (`self.isSwordEquipped?`)
    (set `self.MouseLeftIsPressed` true)
    ;[1 1 1] Stop moving while using sword
    (set `self.isSlashing` true)
    (set `CharacterMovementComponent.MaxWalkSpeed` 0.0 _charactermovement)
    (set `CharacterMovementComponent.RotationRate` (struct) _charactermovement)
    (`KismetSystemLibrary.Delay` 0.5)
    (`GameplayStatics.PlaySound2D` "/Game/Sounds/swordSwing.swordSwing" 1.0 1.0 0.0 null null)))

(event `releaseSwing`
  (bind _charactermovement (`self.CharacterMovement`))
  ;[1 1 1] SwingSword Trigger Mouse Button
  (`KismetSystemLibrary.Delay` 1.0)
  (set `self.MouseLeftIsPressed` false)
  (set `self.isSlashing` false)
  ;[1 1 1] Stop moving while using sword
  (set `CharacterMovementComponent.MaxWalkSpeed` 600.0 _charactermovement)
  (set `CharacterMovementComponent.RotationRate` (struct :`Yaw` 540.0) _charactermovement))

(event `EquipSword`
  (bind _currentweapon (`self.currentWeapon`))
  ;[1 1 1] equip sword
  ;;[1 1 1] press 1
  (if (not (`self.isSlashing`))
    (set `self.isSwordEquipped?` true)
    (`/Engine/EditorBlueprintResources/StandardMacros.IsValid` _currentweapon
      (:`Is Valid`
        (`self.K2_AttachToComponent` _currentweapon (`self.Mesh`) "SwordSocket" "SnapToTarget" "SnapToTarget" "KeepRelative" true)))))

(event `putSwordBack`
  (bind _currentweapon (`self.CurrentWeapon`))
  ;[1 1 1] equip sword
  ;;[1 1 1] press 3
  (if (`self.isSlashing`)
    _
    (elif (not (`self.isInComboMode`))
      (set `self.isSwordEquipped?` false)
      (`/Engine/EditorBlueprintResources/StandardMacros.IsValid` _currentweapon
        (:`Is Valid`
          (`self.K2_AttachToComponent` _currentweapon (`self.Mesh`) "unshealthed" "SnapToTarget" "SnapToTarget" "KeepRelative" true))))))

(event `DropObject`
  ;[1 1 1] PICKUP BOJECT
  ;;[1 1 1] Drop object function
  (`PhysicsHandleComponent.ReleaseComponent` (`self.PhysicsHandle`))
  (set `self.isHoldingObject` false))

(event `Pick`
  (params (Release :type Boolean) (Pick :type Boolean))
  ;[1 1 1] PICKUP BOJECT
  ;;[1 1 1] PICKUP ACTION
  (`self.PickUpDecisionMaker` Release Pick))

(event `PickUpObject`
  ;[1 1 1] PICKUP BOJECT
  ;;[1 1 1] PickUp object function]
  (`self.PickUpMechanism`))

(event `ThrowSword`
  (bind _currentweapon (`self.currentWeapon`))
  (bind _returnvalue (`SceneComponent.GetSocketLocation` (`self.Mesh`) "SwordSocket"))
  (bind (_returnvalue_roll _returnvalue_pitch _returnvalue_yaw) (`KismetMathLibrary.BreakRotator` (`KismetMathLibrary.FindLookAtRotation` (`self.K2_GetActorLocation` _currentweapon) (`self.HitLoc`))))
  ;[1 1 1] THROW SWORD
  ;;[1 1 1] Keyboard Input Check
  (if (`self.isWIthPlayer`)
    (if (not (`self.isInAir`))
      (if (not (`self.isInComboMode`))
        ;;[1 1 1] replace with good sound
        (`GameplayStatics.PlaySound2D` "/Game/Sounds/swordSwing.swordSwing" 1.0 1.0 0.0 null null)
        ;[1 1 1] set walking speed when throwing sword
        (set `CharacterMovementComponent.MaxWalkSpeed` 100.0 (`self.CharacterMovement`))
        (set `self.isHoldingObject` false)
        ;[1 1 1] Trace a line from player to surrounding Target
        (bind (_outhit _returnvalue_2) (`KismetSystemLibrary.LineTraceSingle` _returnvalue (+ _returnvalue (* (`KismetMathLibrary.GetForwardVector` (`SceneComponent.K2_GetComponentRotation` (`self.FollowCamera`))) 10000.0)) "TraceTypeQuery1"))
        (if _returnvalue_2
          ;[1 1 1] set the sword start location (From Location)
          (bind _output_get (set `self.fromLoc` (`self.K2_GetActorLocation` (`self.currentWeapon`))))
          (bind (_bblockinghit _binitialoverlap _time _distance _location _impactpoint) (`GameplayStatics.BreakHitResult` _outhit))
          ;[1 1 1] first find direction of hit location from player by substracting From loc and Hit point which gives a vector, and  setting the impact point by adding the hit point to the resultant vector
          (bind _output_get_2 (set `self.HitLoc` (+ (* (`KismetMathLibrary.Normal` (- _output_get _impactpoint)) 25.0) _impactpoint)))
          ;[1 1 1] Rotating the sword when in air.. set Z-Yaw
          (set `self.heading` (`KismetMathLibrary.Normal` (- _output_get_2 _output_get)))
          (set `self.Rot` (`self.K2_GetActorRotation` _currentweapon))
          (set `self.zYaw` _returnvalue_yaw)
          ;[1 1 1] Finally Detach the sword from actor
          (`self.K2_DetachFromActor` (`self.currentWeapon`) "KeepWorld" "KeepWorld" "KeepWorld")
          ;[1 1 1] set the sword is in air
          (set `self.isInAir` true)
          (set `self.isWIthPlayer` false)
          (set `self.isSwordEquipped?` false))))))

(event `CallSwordBack`
  ;[1 1 1] CALL SWORD BACK
  (if (`self.isWIthPlayer`)
    _
    (elif (not (`self.isInComboMode`))
      ;[1 1 1] Recall function when B pressed
      (set `CharacterMovementComponent.MaxWalkSpeed` 600.0 (`self.CharacterMovement`))
      (if (not (`self.isInAir`))
        (`self.RecallSword`)))))

(event `self.ReceiveTick`
  (params (DeltaSeconds :type "Float (single-precision)"))
  (bind (_rot_roll _rot_pitch _rot_yaw) (`KismetMathLibrary.BreakRotator` (`self.Rot`)))
  (bind _currentweapon (`self.currentWeapon`))
  (bind _halfdistance (`self.HalfDistance`))
  (bind (_rot_roll_2 _rot_pitch_2) (`KismetMathLibrary.BreakRotator` (`self.Rot`)))
  (bind _returnvalue (`KismetMathLibrary.VInterpTo_Constant` (`self.K2_GetActorLocation` (`self.currentWeapon`)) (`self.HitLoc`) DeltaSeconds (`self.AxeSpeed`)))
  (bind _returnvalue_2 (+ (`SceneComponent.GetSocketLocation` (`self.Mesh`) "SwordSocket") (* (`self.GetActorRightVector` _currentweapon) (`KismetMathLibrary.Lerp` _halfdistance 0.0 (`KismetMathLibrary.FClamp` (/ (`KismetMathLibrary.Abs` (- _halfdistance (`self.currentDistance`))) (/ _halfdistance 2.0)))))))
  (`|ExecutionSequence`
    (:`then_0`
      (`self.UpdatePhysicsHandle`))
    (:`then_1`
      ;[1 1 1] check if player is holding weapon
      (if (`self.isHoldingObject`)
        _
        (elif (`self.isInAir`)
          ;[1 1 1] check if the sword is in that threshhold distance, if not set to normal rotation of the sword
          (if (<= (`KismetMathLibrary.VSize` (- (`self.K2_GetActorLocation` (`self.currentWeapon`)) (`self.HitLoc`))) (/ (`self.AxeSpeed`) 2.0))
            ;[1 1 1] if the distance(wall and sword) is less then set the sword to is in air
            (if (< (`KismetMathLibrary.VSize` (- (`self.K2_GetActorLocation` (`self.currentWeapon`)) (`self.HitLoc`))) 5.0)
              (set `self.isInAir` false)
              (else
                ;[1 1 1] if the sword is near enough set the custom rotation to make it seem like exact hit
                (bind _output_get (set `self.Rot` (`KismetMathLibrary.RInterpTo_Constant` (`self.Rot`) (`KismetMathLibrary.MakeRotator` 0.0 -60.0 (`self.zYaw`)) DeltaSeconds (`self.RotationSpeed`))))
                (`self.K2_SetActorLocationAndRotation` (`self.currentWeapon`) _returnvalue _output_get false false)))
            (else
              ;[1 1 1] set actor location and rotation when flying
              (bind _output_get_2 (set `self.Rot` (`KismetMathLibrary.RInterpTo_Constant` (`self.Rot`) (`KismetMathLibrary.MakeRotator` 0.0 (+ _rot_pitch_2 -10.0) (`self.zYaw`)) DeltaSeconds (`self.RotationSpeed`))))
              (`self.K2_SetActorLocationAndRotation` (`self.currentWeapon`) _returnvalue _output_get_2 false false)))
          (else
            ;[1 1 1] If sword is not near ,chek if the sword is returning or not
            (if (`self.return `)
              ;[1 1 1] Node to check if Wepaon is near player when returning back
              (bind _output_get_3 (set `self.currentDistance` (`KismetMathLibrary.VSize` (- (`SceneComponent.GetSocketLocation` (`self.Mesh`) "SwordSocket") (`self.K2_GetActorLocation` (`self.currentWeapon`))))))
              (if (<= _output_get_3 (/ (`self.AxeSpeed`) 2.0))
                ;[1 1 1] BringSword Back
                (bind _output_get_4 (set `self.Rot` (`KismetMathLibrary.RInterpTo_Constant` (`self.Rot`) (`KismetMathLibrary.MakeRotator` 0.0 0.0 (`self.zYaw`)) DeltaSeconds (`self.RotationSpeed`))))
                (`self.K2_SetActorLocationAndRotation` (`self.currentWeapon`) (`KismetMathLibrary.VInterpTo_Constant` (`self.K2_GetActorLocation` (`self.currentWeapon`)) _returnvalue_2 DeltaSeconds (* (`self.AxeSpeed`) 2.0)) _output_get_4 false false)
                (if (< (`self.currentDistance`) 10.0)
                  (set `self.isInAir` false)
                  (set `self.return ` false)
                  (set `self.isWIthPlayer` true)
                  (set `self.isSwordEquipped?` true)
                  (`self.K2_AttachToComponent` (`self.currentWeapon`) (`self.Mesh`) "SwordSocket" "SnapToTarget" "SnapToTarget" "SnapToTarget" true)
                  (`GameplayStatics.PlayWorldCameraShake` null (`SceneComponent.K2_GetComponentLocation` (`self.FollowCamera`)) 0.0 500.0 5.0 true)
                  (`GameplayStatics.PlaySound2D` "/Game/Sounds/Grab.Grab" 1.0 1.0 0.0 null null))
                (else
                  (bind _output_get_5 (set `self.Rot` (`KismetMathLibrary.RInterpTo_Constant` (`self.Rot`) (`KismetMathLibrary.MakeRotator` 0.0 (+ _rot_yaw 10.0) (`self.zYaw`)) DeltaSeconds (`self.RotationSpeed`))))
                  (`self.K2_SetActorLocationAndRotation` (`self.currentWeapon`) (`KismetMathLibrary.VInterpTo_Constant` (`self.K2_GetActorLocation` _currentweapon) _returnvalue_2 DeltaSeconds (`self.AxeSpeed`)) _output_get_5 false false))))))))))

(event `self.BPC_Health.onDeath`
  ;[1 1 1] on Death
  (set `self.IsDead` true)
  (`GameplayStatics.PlaySound2D` "/Game/Sounds/PlayerSound/Cue_PlayerDeath.Cue_PlayerDeath" 1.0 1.0 0.0 null null)
  (`KismetSystemLibrary.Delay` 5.0)
  (`self.RespawnCharacter` (`self.Respawn`))
  (`self.K2_DestroyActor`)
  (set `self.IsDead` false))

(event `set is damaged`
  ;[1 1 1] Is Damaged
  (if (not (`self.IsDead`))
    (`GameplayStatics.PlaySound2D` "/Game/Sounds/PlayerSound/Cue_PlayerHurt.Cue_PlayerHurt" 1.0 1.0 0.0 null null)
    (set `self.isDamaged` true)
    (`KismetSystemLibrary.Delay` 0.5)
    (set `self.isDamaged` false)))

(fn `PickUpDecisionMaker`
  (params (Condition :type Boolean) (Condition2 :type Boolean))
  (bind _charactermovement (`self.CharacterMovement`))
  (bind _charactermovement_2 (`self.CharacterMovement`))
  (bind _returnvalue (not (`NavMovementComponent.IsFalling` (`self.CharacterMovement`))))
  (if Condition
    ;[1 1 1] check before picking object
    (if _returnvalue
      (`|ExecutionSequence`
        (:`then_0`
          ;[1 1 1] When right mouse is pressed set movement and rotation rate to 0
          (if (`self.isSwordEquipped?`)
            (set `self.isSlashing` true)
            (set `self.MouseRight IsPressed` true)
            (set `self.isInComboMode` true)
            (set `CharacterMovementComponent.MaxWalkSpeed` 0.0 _charactermovement)
            (set `CharacterMovementComponent.RotationRate` (struct) _charactermovement)))
        (:`then_1`
          ;[1 1 1] check if it is holding object
          (if (`self.isSwordEquipped?`)
            _
            (elif (not (`self.isHoldingObject`))
              (`self.PickUpObject`))))))
    (elif Condition2
      (if _returnvalue
        (`|ExecutionSequence`
          (:`then_0`
            ;[1 1 1] set rotation and movent back to normal when combo is finshed
            (if (`self.isSwordEquipped?`)
              (set `self.isSlashing` false)
              (set `self.isInComboMode` false)
              (set `self.MouseRight IsPressed` false)
              (set `self.isHoldingObject` true)
              (set `CharacterMovementComponent.MaxWalkSpeed` 600.0 _charactermovement_2)
              (set `CharacterMovementComponent.RotationRate` (struct :`Yaw` 540.0) _charactermovement_2)))
          (:`then_1`
            (if (`self.isHoldingObject`)
              (`self.DropObject`))))))))

(fn `PickUpMechanism`
  (bind _followcamera (`self.FollowCamera`))
  (bind _returnvalue (`SceneComponent.K2_GetComponentLocation` _followcamera))
  (bind (_outhit _returnvalue_2) (`KismetSystemLibrary.LineTraceSingleForObjects` _returnvalue (+ (* (`SceneComponent.GetForwardVector` _followcamera) 500.0) _returnvalue) (`|MakeArray` "ObjectTypeQuery1" :!type "EObjectTypeQuery Enum")))
  (if _returnvalue_2
    (bind (_bblockinghit _binitialoverlap _time _distance _location _impactpoint _normal _impactnormal _physmat _hitactor _hitcomponent) (`GameplayStatics.BreakHitResult` _outhit))
    (if (`SceneComponent.IsSimulatingPhysics` _hitcomponent "None")
      (`PhysicsHandleComponent.GrabComponentAtLocation` (`self.PhysicsHandle`) _hitcomponent "None" (`SceneComponent.K2_GetComponentLocation` _hitcomponent))
      (set `self.isHoldingObject` true))))

(fn `RecallSword`
  (set `self.Rot` (`self.K2_GetActorRotation` (`self.currentWeapon`)))
  (set `self.HalfDistance` (/ (`KismetMathLibrary.VSize` (- (`SceneComponent.GetSocketLocation` (`self.Mesh`) "SwordSocket") (`self.K2_GetActorLocation` (`self.currentWeapon`)))) 2.0))
  (set `self.return ` true)
  (set `self.isInAir` true))

(fn `RespawnCharacter`
  (params (`spawn location` :type "Transform Structure"))
  (bind _returnvalue (`|SpawnActorFromClass` "BP_PlayerChar_C" `spawn location` "Undefined" "OverrideRootScale" null null))
  (`Controller.Possess` (`self.GetController` (`GameplayStatics.GetPlayerCharacter` 0)) _returnvalue)
  (`self.K2_DestroyActor` (`self.currentWeapon`)))

(fn `startTracing`
  (params (newActor :type "Actor Object Reference") (oldActor :type "Actor Object Reference"))
  ;[1 1 1] draw on new and remove on old
  (`PrimitiveComponent.SetRenderCustomDepth` (`|GetArrayItem` (`self.GetComponentsByTag` newActor "/Script/Engine.PrimitiveComponent" "outline")) true)
  (if (not (== oldActor null))
    (`PrimitiveComponent.SetRenderCustomDepth` (`|GetArrayItem` (`self.GetComponentsByTag` oldActor "/Script/Engine.PrimitiveComponent" "outline")) false)))

(fn `stopTracing`
  (bind (_interactable_bblockinghit _interactable_binitialoverlap _interactable_time _interactable_distance _interactable_location _interactable_impactpoint _interactable_normal _interactable_impactnormal _interactable_physmat _interactable_hitactor) (`GameplayStatics.BreakHitResult` (`self.interactable`)))
  (`|ExecutionSequence`
    (:`then_0`
      (if (!= _interactable_hitactor null)
        (`PrimitiveComponent.SetRenderCustomDepth` (`|GetArrayItem` (`self.GetComponentsByTag` _interactable_hitactor "/Script/Engine.PrimitiveComponent" "outline")) false)))
    (:`then_1`
      (set `self.interactable` (struct)))))

(fn `UpdatePhysicsHandle`
  ;[1 1 1] usage of physics handle to hold object (Pick up function)
  (`PhysicsHandleComponent.SetTargetLocation` (`self.PhysicsHandle`) (`SceneComponent.K2_GetComponentLocation` (`self.HoldObject`))))

(fn `UserConstructionScript`)