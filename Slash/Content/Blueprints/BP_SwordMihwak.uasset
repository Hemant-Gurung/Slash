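; BP_SwordMihwak is a melee sword that deals DamageAmount through a Box overlap.
; Overlaps call IsHurt on Enemy-tagged BP_EnemyChar actors and damage their BPC_Health; BP_DamagebleActor props take damage through their own health component.
; The Box starts without collision, and Tick enables it one second after detecting a player mouse press, disabling it when neither button is held.
; IsInAir forces collision on.
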(event `self.ReceiveBeginPlay`
  (`PrimitiveComponent.SetCollisionEnabled` (`self.Box`) "NoCollision"))

(event `self.Box.OnComponentBeginOverlap`
  (params (OverlappedComponent :type "PrimitiveComponent Object Reference") (OtherActor :type "Actor Object Reference") (OtherComp :type "PrimitiveComponent Object Reference") (OtherBodyIndex :type Integer) (bFromSweep :type Boolean) (SweepResult :type "HitResult Structure (by ref)"))
  (bind _returnvalue (`self.GetComponentByClass` OtherActor "/Game/Blueprints/BPC_Health.BPC_Health_C"))
  (`/Engine/EditorBlueprintResources/StandardMacros.IsValid` OtherActor
    (:`Is Valid`
      (`|ExecutionSequence`
        (:`then_0`
          (if (`self.ActorHasTag` OtherActor "Enemy")
            (bind _asbp_enemy_char (cast `/Game/Blueprints/BP_EnemyChar` OtherActor))
            (`/Game/Blueprints/BP_EnemyChar.IsHurt` _asbp_enemy_char)
            ;[1 1 1] if valid do damage
            (`/Engine/EditorBlueprintResources/StandardMacros.IsValid` _returnvalue
              (:`Is Valid`
                (`/Game/Blueprints/BPC_Health.DoDamage` _returnvalue (`self.Damage Amount`))))))
        (:`then_1`
          (bind _asbp_damageble_actor (cast `/Game/Blueprints/BP_DamagebleActor` OtherActor))
          (`/Game/Blueprints/BPC_Health.DoDamage` (`/Game/Blueprints/BP_DamagebleActor.BPC_Health` _asbp_damageble_actor) (`self.Damage Amount`)))))))

(event `self.ReceiveTick`
  (params (DeltaSeconds :type "Float (single-precision)"))
  (bind _returnvalue (`GameplayStatics.GetPlayerCharacter` 0))
  (`|ExecutionSequence`
    (:`then_0`
      ;[1 1 1] check for damage only when button is pressed
      (bind _asbp_player_char (cast `/Game/Blueprints/BP_PlayerChar` _returnvalue))
      (`/Engine/EditorBlueprintResources/StandardMacros.IsValid` _returnvalue
        (:`Is Valid`
          (if (or (`/Game/Blueprints/BP_PlayerChar.MouseLeftIsPressed` _asbp_player_char) (`/Game/Blueprints/BP_PlayerChar.MouseRight IsPressed` _asbp_player_char))
            (`KismetSystemLibrary.Delay` 1.0)
            (`PrimitiveComponent.SetCollisionEnabled` (`self.Box`) "QueryAndPhysics")
            (else
              (`PrimitiveComponent.SetCollisionEnabled` (`self.Box`) "NoCollision"))))))
    (:`then_1`
      (if (`self.isInAir`)
        (`PrimitiveComponent.SetCollisionEnabled` (`self.Box`) "QueryAndPhysics")))))

(fn `UserConstructionScript`)